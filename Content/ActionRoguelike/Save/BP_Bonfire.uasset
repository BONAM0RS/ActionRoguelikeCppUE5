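; Bonfire interactable that acts as a save point, lighting its fire and saving the world when used.
; Interact sets FireActive, writes the save through the RL save game subsystem, activates the fire particles and prints a confirmation.
; OnActorLoaded reapplies the lit state from FireActive after a load.
; The interact prompt text is left empty.
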(event Custom|Update%20Bonfire
  (if (Variables|Default|GetbFireActive)
    (Components|Activation|Activate (Variables|Default|GetParticleSystem) false)))

(event EventBeginPlay)

(event Collision|EventActorBeginOverlap
  (params (OtherActor :type Actor%20Object%20Reference)))

(event EventTick
  (params (DeltaSeconds :type Float%20%28single-precision%29)))

(event EventInteract
  (params (InstigatorPawn :type Pawn%20Object%20Reference))
  (Variables|Default|SetbFireActive true)
  (Class|RLSaveGameSubsystem|WriteSaveGame (Subsystems|GetRLSaveGameSubsystem))
  (CallFunction|UpdateBonfire)
  (Development|PrintString "WORLD SAVED" true true "(R=0.000000,G=1.000000,B=0.039678,A=1.000000)"))

(event EventOnActorLoaded
  (CallFunction|UpdateBonfire))

(fn ConstructionScript)

(fn GetInteractText
  (params (InstigatorPawn :type Pawn%20Object%20Reference))
  (return ""))