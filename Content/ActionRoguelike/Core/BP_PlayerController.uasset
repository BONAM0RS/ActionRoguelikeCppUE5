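; Player controller for the ActionRoguelike game that sets up the local player's HUD and offers a manual save key.
; When play state begins on a local controller, it creates the W_HUD widget, adds it to the viewport and switches to game-only input.
; Pressing L casts the game mode to RLGameModeBase, writes the save game and prints a confirmation.
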(event EventBeginPlay)

(event EventBlueprintBeginPlayingState
  (if (Pawn|IsLocalController)
    (bind _returnvalue (UserInterface|CreateWidget "/Game/ActionRoguelike/UI/Widgets/HUD/W_HUD.W_HUD_C"))
    (UserInterface|Viewport|AddtoViewport _returnvalue 0)
    (Input|SetInputModeGameOnly self false)))

(event Input|KeyboardEvents|L
  (params (Key :type Key%20Structure :default "None"))
  (:Pressed
    (bind _asrlgame_mode_base (Utilities|Casting|CastToRLGameModeBase (Game|GetGameMode)))
    (Class|RLGameModeBase|WriteSaveGame _asrlgame_mode_base)
    (Development|PrintString "WORLD SAVED")))

(fn ConstructionScript)