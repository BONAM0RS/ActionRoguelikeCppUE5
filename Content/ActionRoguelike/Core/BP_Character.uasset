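; Player character Blueprint for an action roguelike that creates the W_HUD widget on BeginPlay and prototypes a primary projectile attack.
; SpawnProjectile traces from the camera along its forward vector with debug drawing to find an aim point.
; It spawns the projectile at the muzzle socket rotated toward that point, so shots converge on the camera's aim.
; Overlap and health-change events are empty; montage, timer and debug-print nodes are disconnected.
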(event OnComponentBeginOverlap(CapsuleComponent)
  (params (OverlappedComponent :type Primitive%20Component%20Object%20Reference) (OtherActor :type Actor%20Object%20Reference) (OtherComp :type Primitive%20Component%20Object%20Reference) (OtherBodyIndex :type Integer) (bFromSweep :type Boolean) (SweepResult :type Hit%20Result%20Structure%20%28by%20ref%29)))

(event OnHealthChanged(AttributeComponent)
  (params (InstigatorActor :type Actor%20Object%20Reference) (OwningComponent :type RL%20Attribute%20Component%20Object%20Reference) (NewHalth :type Float%20%28single-precision%29) (Delta :type Float%20%28single-precision%29)))

(event Custom|Spawn%20Projectile
  (bind _cameracomponent (Variables|Default|GetCameraComponent))
  (bind _mesh (Variables|Character|GetMesh))
  (bind _returnvalue (Transformation|GetSocketLocation _mesh "Muzzle_01"))
  ;[1 1 1] Primary Attack prototyping
  (bind _output_get (Variables|Default|SetEnd (+ (Transformation|GetWorldLocation _cameracomponent) (* (Math|Vector|GetForwardVector (Transformation|GetWorldRotation _cameracomponent)) (Math|Float|MakeLiteralFloat 5e+03)))))
  (bind (_outhit _returnvalue_2) (Collision|LineTraceForObjects (Transformation|GetWorldLocation (Variables|Default|GetCameraComponent)) _output_get (Variables|Default|GetObject%20Types) false 0 "ForDuration"))
  (if _returnvalue_2
    (Variables|Default|SetEnd (.ImpactPoint (Collision|BreakHitResult _outhit))))
  (Game|SpawnActorfromClass (Variables|Default|GetPrimaryProjectileClass) (Math|Transform|MakeTransform _returnvalue (Math|Rotator|FindLookatRotation _returnvalue (Variables|Default|GetEnd)) "1.000000,1.000000,1.000000") "AlwaysSpawn" "MultiplyWithRoot" 0 self))

(event EventBeginPlay
  (bind _returnvalue (UserInterface|CreateWidget "/Game/ActionRoguelike/UI/Widgets/W_HUD.W_HUD_C"))
  (UserInterface|Viewport|AddtoViewport _returnvalue 0))

(event Input|ActionEvents|InputActionPrimaryAttack
  (params (Key :type Key%20Structure :default "None"))
  ;[1 1 1] Primary Attack prototyping
)

(fn ConstructionScript)