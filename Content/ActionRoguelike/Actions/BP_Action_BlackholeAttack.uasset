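; Blackhole attack action that costs Rage from the instigator's attributes.
; CanStart adds a Rage check on top of the parent's conditions and prints an on-screen warning when Rage is too low.
; StartAction subtracts the Rage cost through the attribute component, then runs the parent start logic, which carries out the rest of the attack.
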(event EventStartAction
  (params (Instigator :type Actor%20Object%20Reference))
  (bind _returnvalue (Class|RLAttributeComponent|GetAttributes Instigator))
  (Class|RLAttributeComponent|ApplyRageChange _returnvalue Instigator (/ (Variables|Default|GetRage%20Cost) -1.0))
  (|CallParentFunction Instigator))

(fn CanStart
  (params (Instigator :type Actor%20Object%20Reference))
  (bind _returnvalue (|CallParentFunction Instigator))
  (if _returnvalue
    (bind _returnvalue_2 (Class|RLAttributeComponent|GetAttributes Instigator))
    (if (>= (Class|RLAttributeComponent|GetCurrentRage _returnvalue_2) (Variables|Default|GetRage%20Cost))
      (return true)
      (else
        (Development|PrintString "Not enough Rage: take damage to get rage" true true "(R=1.000000,G=0.039770,B=0.009923,A=1.000000)")
        (return false)))
    (else
      (return false))))