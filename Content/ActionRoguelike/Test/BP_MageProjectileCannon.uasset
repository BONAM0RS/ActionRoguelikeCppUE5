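; BP_MageProjectileCannon is a test cannon actor that fires projectiles from an Arrow component on a looping timer when Attack is enabled.
; Each spawned projectile receives a damage amount, optionally re-rolled per shot as a random integer between configurable minimum and maximum values.
; When FollowPlayer is set, Tick rotates the static mesh toward the player pawn using MakeRotFromX on the direction vector.
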(event Custom|Shoot%20Projectile
  (bind _arrow (Variables|Default|GetArrow))
  (if (not (Variables|Default|GetbRandomDamage))
    _
    (else
      (Variables|Default|SetDamageAmount (Math|Conversions|ToFloat(Integer) (Math|Random|RandomIntegerinRange (Math|Float|Truncate (Variables|Default|GetMinDamageAmount)) (Math|Float|Truncate (Variables|Default|GetMaxDamageAmount)))))))
  (Game|SpawnActorfromClass "/Game/ActionRoguelike/Projectiles/BP_MageProjectile.BP_MageProjectile_C" (Math|Transform|MakeTransform (Transformation|GetWorldLocation _arrow) (Transformation|GetWorldRotation _arrow) "1.000000,1.000000,1.000000") "Undefined" "MultiplyWithRoot" 0 (Variables|Default|GetDamageAmount) 0))

(event EventBeginPlay
  (if (Variables|Default|GetbAttack)
    (Utilities|Time|SetTimerbyEvent (delegate Custom|Shoot%20Projectile) 2.0 true)))

(event EventTick
  (params (DeltaSeconds :type Float%20%28single-precision%29))
  (if (Variables|Default|GetbFollowPlayer)
    (Transformation|SetWorldRotation (Variables|Default|GetStaticMesh) (Math|Rotator|MakeRotfromX (- (Transformation|GetActorLocation (Game|Player|GetPlayerPawn 0)) (Transformation|GetActorLocation))) false false)))

(fn ConstructionScript)