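; BP_ItemChest is a test item chest Blueprint whose Interact event only forwards to the parent implementation.
; BeginPlay, Tick and the construction script are empty.
; Disconnected leftovers hold debug prints, a gameplay tag check against RLActionComponent for a required key card, and a FlipFlop-driven timeline that pitches the lid open or closed and activates particles once it finishes.
; None of that leftover logic runs.
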(event EventBeginPlay)

(event EventInteract
  (params (InstigatorPawn :type Pawn%20Object%20Reference))
  (|CallParentFunction InstigatorPawn))

(event EventTick
  (params (DeltaSeconds :type Float%20%28single-precision%29)))

(fn ConstructionScript)