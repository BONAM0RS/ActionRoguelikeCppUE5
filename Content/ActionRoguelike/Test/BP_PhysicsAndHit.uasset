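; BP_PhysicsAndHit is a test actor that reacts to damage through its RLAttribute component's health-change event.
; While health stays above zero, each change spawns a W_DamagePopUp widget attached to the actor, showing the delta.
; It also writes the current time to the mesh material's TimeToHit parameter, so the shader can time a hit effect.
; When health reaches zero or below, the actor destroys itself.
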(event OnHealthChanged(RLAttribute)
  (params (InstigatorActor :type Actor%20Object%20Reference) (OwningComponent :type RL%20Attribute%20Component%20Object%20Reference) (NewValue :type Float%20%28single-precision%29) (Delta :type Float%20%28single-precision%29))
  (if (not (<= NewValue 0.0))
    (bind _returnvalue (UserInterface|CreateWidget "/Game/ActionRoguelike/UI/Widgets/World/W_DamagePopUp.W_DamagePopUp_C" 0 self (Utilities|Text|ToText(Float) Delta "HalfToEven")))
    (UserInterface|Viewport|AddtoViewport _returnvalue 0)
    (Rendering|Material|SetScalarParameterValueonMaterials (Variables|Debug|GetStaticMeshComponent) "TimeToHit" (Utilities|Time|GetTimeSeconds))
    (else
      (Actor|DestroyActor))))

(event EventBeginPlay)

(fn ConstructionScript)