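; BP_Lever is a test interactable lever that grants a key card gameplay tag to whoever uses it.
; On Interact it tilts the handle mesh to a fixed rotation and adds the tag directly to the instigator's RLActionComponent active tags.
; Its interact text is empty, and the event graph keeps two unconnected examples contrasting an interact message with a cast to an explosive barrel.
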(event EventBeginPlay)

(event EventInteract
  (params (InstigatorPawn :type Pawn%20Object%20Reference))
  (Transformation|SetRelativeRotation (Variables|Default|GetHandleMesh) "-30.000000,0.000000,0.000000" false false)
  (GameplayTags|AddGameplayTag (Variables|/Script/ActionRoguelike.RLActionComponent|GetActiveGameplayTags (Actor|GetComponentbyClass InstigatorPawn "/Script/ActionRoguelike.RLActionComponent")) (Variables|Default|GetKeyCardTag) :!class /Script/GameplayTags.BlueprintGameplayTagLibrary))

(fn ConstructionScript)

(fn GetInteractText
  (params (InstigatorPawn :type Pawn%20Object%20Reference))
  (return ""))