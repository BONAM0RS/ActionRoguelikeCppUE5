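; BP_ItemChest is an interactable item chest Blueprint that hands Interact straight to its parent implementation.
; Tick prints the LidOpened state to screen every frame as a debug readout.
; Unconnected leftover nodes hold an interact print, a key card GameplayTag check on an RLActionComponent, and a FlipFlop timeline that pitches the lid and activates particles.
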(event EventBeginPlay)

(event EventInteract
  (params (InstigatorPawn :type Pawn%20Object%20Reference))
  (|CallParentFunction InstigatorPawn))

(event EventTick
  (params (DeltaSeconds :type Float%20%28single-precision%29))
  (Development|PrintString (Utilities|String|ToString(Boolean) (Variables|Default|GetbLidOpened)) true true "(R=1.000000,G=0.406657,B=0.000000,A=1.000000)" 0.0))

(fn ConstructionScript)